(event `launch_session`
  (`CreateSessionCallbackProxy.CreateSession` (`GameplayStatics.GetPlayerController` 0) 5 true
    (:`OnSuccess`
      (`GameplayStatics.OpenLevel` "test" true "listen"))
    (:`OnFailure`
      (`KismetSystemLibrary.PrintString` "failed to create session"))))

(event `connect_session`
  (bind _results (`FindSessionsCallbackProxy.FindSessions` (`GameplayStatics.GetPlayerController` 0) 5 true)
    (:`OnSuccess`
      (`KismetSystemLibrary.PrintString` "session found")
      (for _array_element _results
        (`JoinSessionCallbackProxy.JoinSession` (`GameplayStatics.GetPlayerController` 0) _array_element
          (:`OnSuccess`
            (break))))
      (`GameplayStatics.OpenLevel` "test"))
    (:`OnFailure`
      (`KismetSystemLibrary.PrintString` "sessions not found"))))