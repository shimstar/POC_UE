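; Player pawn for a networked game, flown as a physics-driven mesh with throttle, pitch and yaw, plus health.
; The locally controlled pawn sends force and torque through events that act only on authority, which then passes the mesh transform on, while remote copies disable physics.
; Bullet overlaps, matched by display name, are detected locally and trigger damage, destroying the pawn at zero health.
; Collisions reset speed on authority.
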(event `self.ReceiveBeginPlay`
  ;[1 1 1] disable physic on client
  (`/Engine/EditorBlueprintResources/ActorMacros.Switch Has Authority`
    (:`Remote`
      (`PrimitiveComponent.SetSimulatePhysics` (`self.StaticMesh`) false))))

(event `InputAxis|speed`
  (params (AxisValue :type "Float (single-precision)"))
  (bind _returnvalue (+ (`self.speed`) (* AxisValue 15.0)))
  ;[1 1 1] speed
  (if (`self.IsLocallyControlled`)
    (if (<= _returnvalue (`self.speedmax`))
      (if (>= _returnvalue -150.0)
        (set `self.speed` _returnvalue)))))

(event `self.ReceiveTick`
  (params (DeltaSeconds :type "Float (single-precision)"))
  ;[1 1 1] move forward
  (if (`self.IsLocallyControlled`)
    (`self.servermoveforward_Event` (* (`SceneComponent.GetForwardVector` (`self.StaticMesh`)) (* (`self.speed`) -1.0)))))

(event `servermoveforward_Event`
  (params (value :type "Vector Structure"))
  (bind _staticmesh (`self.StaticMesh`))
  ;[1 1 1] move forward
  (`/Engine/EditorBlueprintResources/ActorMacros.Switch Has Authority`
    (:`Authority`
      (`PrimitiveComponent.AddForce` (`self.StaticMesh`) value "None" true)
      (`self.setlocation_Event` (`SceneComponent.K2_GetComponentLocation` _staticmesh) (`SceneComponent.K2_GetComponentRotation` _staticmesh)))))

(event `InputAxis|leftright`
  (params (AxisValue :type "Float (single-precision)"))
  ;[1 1 1] manage orque
  (if (`self.IsLocallyControlled`)
    (`self.ADDtorque_Event` (* (`SceneComponent.GetUpVector` (`self.StaticMesh`)) (* AxisValue 3.0)))))

(event `setlocation_Event`
  (params (location :type "Vector Structure") (rotation :type "Rotator Structure"))
  ;[1 1 1] move forward
  (`SceneComponent.K2_SetWorldLocationAndRotation` (`self.StaticMesh`) location rotation false false))

(event `self.ReceiveActorBeginOverlap`
  (params (OtherActor :type "Actor Object Reference"))
  ;[1 1 1] Comment
  (if (>= (`KismetStringLibrary.FindSubstring` (`KismetSystemLibrary.GetDisplayName` OtherActor) "bullet") 0)
    (if (`self.IsLocallyControlled`)
      (bind _asgreen_bullet_bp (cast `/Game/bp/green_bullet_bp` OtherActor))
      (`self.eventdamageserver_Event` (`/Game/bp/green_bullet_bp.damage` _asgreen_bullet_bp))
      (`/Game/bp/green_bullet_bp.overlap_server` _asgreen_bullet_bp))))

(event `ADDtorque_Event`
  (params (val :type "Vector Structure"))
  ;[1 1 1] manage orque
  (`/Engine/EditorBlueprintResources/ActorMacros.Switch Has Authority`
    (:`Authority`
      (`PrimitiveComponent.AddTorque` (`self.StaticMesh`) val "None" true))))

(event `InputAxis|updwon`
  (params (AxisValue :type "Float (single-precision)"))
  ;[1 1 1] manage orque
  (if (`self.IsLocallyControlled`)
    (`self.ADDtorque_Event` (* (`SceneComponent.GetRightVector` (`self.StaticMesh`)) (* AxisValue 3.0)))))

(event `eventdamageserver_Event`
  (params (damage :type "Float (double-precision)"))
  ;[1 1 1] Comment
  (bind _output_get (set `self.health` (- (`self.health`) damage)))
  (if (<= _output_get 0.0)
    (bind _astestgc_bp (cast `/Game/bp/testgc_bp` (`self.GetController` self)))
    (`/Game/bp/testgc_bp.destroy_pawn` _astestgc_bp)
    (`self.K2_DestroyActor` self)))

(event `self.ReceiveHit`
  (params (MyComp :type "PrimitiveComponent Object Reference") (Other :type "Actor Object Reference") (OtherComp :type "PrimitiveComponent Object Reference") (bSelfMoved :type Boolean) (HitLocation :type "Vector Structure") (HitNormal :type "Vector Structure") (NormalImpulse :type "Vector Structure") (Hit :type "HitResult Structure (by ref)"))
  ;[1 1 1] reduce speed to zero on hit
  (`/Engine/EditorBlueprintResources/ActorMacros.Switch Has Authority`
    (:`Authority`
      (set `self.speed` 0.0))))

(fn `UserConstructionScript`)